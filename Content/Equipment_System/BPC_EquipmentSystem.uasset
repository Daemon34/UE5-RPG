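; Equipment system component for the third-person character that handles item pickup and the equipment menu.
; On interact, it sphere-traces from the follow camera, adds a hit BP_Item's data to its inventory array and destroys the actor.
; The menu input toggles the equipment widget, switching cursor and input mode and disabling attacks through the attack component while open.
; A debug key prints the stored item row names.
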(event Input|EnhancedActionEvents|EnhancedInputActionIA_Interact
  (params (ActionValue :type Boolean) (ElapsedSeconds :type Float%20%28double-precision%29) (TriggeredSeconds :type Float%20%28double-precision%29) (InputAction :type Input%20Action%20Object%20Reference :default "/Game/ThirdPerson/Input/Actions/IA_Interact.IA_Interact"))
  (bind _follow_camera (Variables|Default|GetFollow%20Camera))
  (bind _returnvalue (Transformation|GetWorldLocation _follow_camera))
  ;[0.05127 0.05127 0.05127] Pick Up Trace
  (:Started
    (bind (_outhit _returnvalue_2) (Collision|SphereTraceForObjects _returnvalue (+ _returnvalue (* (Math|Vector|GetForwardVector (Transformation|GetWorldRotation _follow_camera)) 1e+03)) 15.0 (Utilities|Array|MakeArray "ObjectTypeQuery2") false 0 "ForDuration"))
    (if _returnvalue_2
      (bind _asbp_item (Utilities|Casting|CastToBP_Item (.HitActor (Collision|BreakHitResult _outhit))))
      (CallFunction|AddItem (Variables|/Game/Equipment_System/BP_Item.BP_Item_C|GetItemData _asbp_item))
      (Actor|DestroyActor _asbp_item)
      (Development|PrintString "Item Gathered"))))

(event Input|EnhancedActionEvents|EnhancedInputActionIA_Menu_Equipment
  (params (ActionValue :type Boolean) (ElapsedSeconds :type Float%20%28double-precision%29) (TriggeredSeconds :type Float%20%28double-precision%29) (InputAction :type Input%20Action%20Object%20Reference :default "/Game/ThirdPerson/Input/Actions/IA_Menu_Equipment.IA_Menu_Equipment"))
  (bind _returnvalue (Game|GetPlayerController 0))
  (bind _returnvalue_2 (Components|GetOwner))
  ;[0.05127 0.05127 0.05127] Equipment Menu Panel
  (:Started
    (if (Variables|Default|GetIsPanelOpened)
      (bind _equipmentwidget (Variables|Default|GetEquipmentWidget)
        (:then
          (Widget|RemovefromParent _equipmentwidget)
          (Variables|Default|SetEquipmentWidget 0)
          (Variables|/Script/Engine.PlayerController|SetbShowMouseCursor _returnvalue false)
          (Input|SetInputModeGameOnly _returnvalue false)
          (bind _asbp_third_person_character (Utilities|Casting|CastToBP_ThirdPersonCharacter _returnvalue_2))
          (Variables|/Game/Blueprints/BPC_AttackSystem.BPC_AttackSystem_C|SetCan%20Attack (Variables|/Game/ThirdPerson/Blueprints/BP_ThirdPersonCharacter.BP_ThirdPersonCharacter_C|GetBPC_AttackSystem _asbp_third_person_character) true)
          (Variables|Default|SetIsPanelOpened false))
        (:else))
      (else
        (bind _returnvalue_3 (UserInterface|CreateWidget "/Game/Equipment_System/UI/WB_Equipment.WB_Equipment_C"))
        (bind _output_get (Variables|Default|SetEquipmentWidget _returnvalue_3))
        (UserInterface|Viewport|AddtoViewport _output_get 0)
        (Variables|/Script/Engine.PlayerController|SetbShowMouseCursor _returnvalue true)
        (Input|SetInputModeGameandUI _returnvalue (Variables|Default|GetEquipmentWidget) "DoNotLock" true false)
        (bind _asbp_third_person_character_2 (Utilities|Casting|CastToBP_ThirdPersonCharacter _returnvalue_2))
        (Variables|/Game/Blueprints/BPC_AttackSystem.BPC_AttackSystem_C|SetCan%20Attack (Variables|/Game/ThirdPerson/Blueprints/BP_ThirdPersonCharacter.BP_ThirdPersonCharacter_C|GetBPC_AttackSystem _asbp_third_person_character_2) false)
        (Variables|Default|SetIsPanelOpened true)))))

(event EventBeginPlay
  (bind _asbp_third_person_character (Utilities|Casting|CastToBP_ThirdPersonCharacter (Components|GetOwner)))
  (Variables|Default|SetFollow%20Camera (Variables|/Game/ThirdPerson/Blueprints/BP_ThirdPersonCharacter.BP_ThirdPersonCharacter_C|GetFollowCamera _asbp_third_person_character)))

(event Input|KeyboardEvents|DebugKeyH
  (params (Key :type Key%20Structure :default "None") (ActionValue :type Input%20Action%20Value%20Structure))
  ;[0.05127 0.05127 0.05127] Pick Up Trace
  (:Pressed
    (for _array_element (Variables|Default|GetInventorySlots)
      (Development|PrintString (Utilities|String|ToString(Name) (.rowname (.item _array_element)))))))

(fn AddItem
  (params (NewItem :type S%20Slots%20Structure%20%28by%20ref%29))
  (Utilities|Array|Add (Variables|Default|GetInventorySlots) NewItem))